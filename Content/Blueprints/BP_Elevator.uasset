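; BP_Elevator is an interactable actor that shows a prompt widget and takes player input while something overlaps its BoxCheck volume.
; Leaving the volume hides the widget and disables input again; overlaps are not filtered by actor type.
; Pressing F calls AdjustWin on the first BP_ThirdPersonCharacterDefault1 found in the world, then plays the WBP_Smash widget's Highlight animation.
; The file contains no elevator movement logic.
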(event `self.ReceiveBeginPlay`
  (`SceneComponent.SetVisibility` (`self.Widget`) false false))

(event `self.BoxCheck.OnComponentBeginOverlap`
  (params (OverlappedComponent :type "PrimitiveComponent Object Reference") (OtherActor :type "Actor Object Reference") (OtherComp :type "PrimitiveComponent Object Reference") (OtherBodyIndex :type Integer) (bFromSweep :type Boolean) (SweepResult :type "HitResult Structure (by ref)"))
  (`SceneComponent.SetVisibility` (`self.Widget`) true false)
  (`self.EnableInput` (`GameplayStatics.GetPlayerController` 0)))

(event `Key|F`
  (params (Key :type "Key Structure"))
  (:`Pressed`
    (`|ExecutionSequence`
      (:`then_0`
        (bind _outactors (`GameplayStatics.GetAllActorsOfClass` "/Game/ThirdPerson/Blueprints/BP_ThirdPersonCharacterDefault1.BP_ThirdPersonCharacterDefault1_C"))
        (`/Game/ThirdPerson/Blueprints/BP_ThirdPersonCharacterDefault1.adjust win` (`|GetArrayItem` _outactors)))
      (:`then_1`
        (bind _aswbp_smash (cast `/Game/Widget/Elevetor/WBP_Smash` (`WidgetComponent.GetWidget` (`self.Widget`))))
        (`UserWidget.PlayAnimation` _aswbp_smash (`/Game/Widget/Elevetor/WBP_Smash.Highlight` _aswbp_smash) 0.0 1 "Forward" 1.0 false)))))

(event `self.BoxCheck.OnComponentEndOverlap`
  (params (OverlappedComponent :type "PrimitiveComponent Object Reference") (OtherActor :type "Actor Object Reference") (OtherComp :type "PrimitiveComponent Object Reference") (OtherBodyIndex :type Integer))
  (`SceneComponent.SetVisibility` (`self.Widget`) false false)
  (`self.DisableInput` (`GameplayStatics.GetPlayerController` 0)))

(fn `UserConstructionScript`)