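; BP_MyWindow_2 is an interactive living-room window that the player slides open and closed with F.
; Box overlap by player character 0 enables the actor's input; end overlap calls DisableInput on the player controller.
; A FlipFlop plays or reverses a timeline that lerps the mesh's relative X from its BeginPlay position to zero, keeping the cached Y.
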(event `self.ReceiveBeginPlay`
  (bind (_relativelocation_x _relativelocation_y) (`KismetMathLibrary.BreakVector` (`SceneComponent.RelativeLocation` (`self.SM_Livingroom_SM_WIndow_02`))))
  (set `self.Relative Location X` _relativelocation_x)
  (set `self.Relative Location Y` _relativelocation_y))

(event `Key|F`
  (params (Key :type "Key Structure"))
  (:`Pressed`
    (`/Engine/EditorBlueprintResources/StandardMacros.FlipFlop`
      (:`A`
        (set `self.IsDoorOpen` true)
        (bind (_direction _newtrack_0) (`Timeline|Timeline_0` :!via `PlayFromStart` :!label _label)
          (:`Update`
            (`SceneComponent.K2_SetRelativeLocation` (`self.SM_Livingroom_SM_WIndow_02`) (`KismetMathLibrary.MakeVector` (`KismetMathLibrary.Lerp` (`self.Relative Location X`) 0.0 _newtrack_0) (`self.Relative Location Y`)) false false))))
      (:`B`
        (set `self.IsDoorOpen` false)
        (goto _label :!via `Reverse`)))))

(event `self.Box.OnComponentBeginOverlap`
  (params (OverlappedComponent :type "PrimitiveComponent Object Reference") (OtherActor :type "Actor Object Reference") (OtherComp :type "PrimitiveComponent Object Reference") (OtherBodyIndex :type Integer) (bFromSweep :type Boolean) (SweepResult :type "HitResult Structure (by ref)"))
  (if (== (`GameplayStatics.GetPlayerCharacter` 0) OtherActor)
    (`self.EnableInput` (`GameplayStatics.GetPlayerController` 0))))

(event `self.Box.OnComponentEndOverlap`
  (params (OverlappedComponent :type "PrimitiveComponent Object Reference") (OtherActor :type "Actor Object Reference") (OtherComp :type "PrimitiveComponent Object Reference") (OtherBodyIndex :type Integer))
  (if (== (`GameplayStatics.GetPlayerCharacter` 0) OtherActor)
    (`self.DisableInput` (`GameplayStatics.GetPlayerController` 0) null)))

(fn `UserConstructionScript`)